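; Lock actor that lights up when its linked key actor reports that the key is found.
; The construction script puts a dynamic instance of the key mesh's material on the lock mesh, so the lock shares the key's material.
; BeginPlay turns that instance's Glow parameter off and binds to the key's KeyFound event, whose handler raises Glow.
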(event `self.ReceiveBeginPlay`
  (`MaterialInstanceDynamic.SetScalarParameterValue` (`self.Lock_Material`) "Glow" 0.0)
  (add `/Game/Keys/BP_Key_Actor.KeyFound` (`self.Key_Actor`) (delegate `KeyFound`)))

(event `KeyFound`
  (`MaterialInstanceDynamic.SetScalarParameterValue` (`self.Lock_Material`) "Glow" 100.0))

(fn `UserConstructionScript`
  (bind _returnvalue (`PrimitiveComponent.CreateDynamicMaterialInstance` (`self.Lock_Mesh`) 0 (`PrimitiveComponent.GetMaterial` (`/Game/Keys/BP_Key_Actor.Key_Mesh` (`self.Key_Actor`)) 0) "None"))
  (set `self.Lock_Material` _returnvalue))